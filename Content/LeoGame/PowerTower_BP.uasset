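; PowerTower_BP is a tower actor that automatically fires MagicProjectile_BP projectiles.
; A looping timer set on BeginPlay calls Shoot every 1.5 seconds, spawning a projectile at the actor's own location and rotation.
; Tick is empty, and an unconnected node that would rotate the Sphere along the player-to-tower direction never runs, so the tower does not track the player.
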(event `self.ReceiveBeginPlay`
  (`KismetSystemLibrary.K2_SetTimerDelegate` (delegate `shoot`) 1.5 true))

(event `self.ReceiveTick`
  (params (DeltaSeconds :type "Float (single-precision)"))
  ;[1 1 1] problem
)

(event `shoot`
  (`|SpawnActorFromClass` "/Game/LeoGame/MagicProjectile_BP.MagicProjectile_BP_C" (`KismetMathLibrary.MakeTransform` (`self.K2_GetActorLocation`) (`self.K2_GetActorRotation`)) "Undefined" "OverrideRootScale" null null))

(fn `UserConstructionScript`)