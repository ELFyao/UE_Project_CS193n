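; Player controller that sets up the main HUD and provides a keyboard shortcut for saving the game.
; On BeginPlay, only the local controller creates the Main_HUD widget, adds it to the viewport and switches to game-only input.
; Pressing L casts the game mode to SGameModeBase, calls WriteSaveGame and prints a success message without checking the result.
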(event `self.ReceiveBeginPlay`
  (if (`self.IsLocalController`)
    (bind _returnvalue (`|CreateWidget` "/Game/LeoGame/UI/Main_HUD.Main_HUD_C"))
    (`UserWidget.AddToViewport` _returnvalue 0)
    (`WidgetBlueprintLibrary.SetInputMode_GameOnly` self)))

(event `Key|L`
  (params (Key :type "Key Structure"))
  (:`Pressed`
    (bind _assgame_mode_base (cast `SGameModeBase` (`GameplayStatics.GetGameMode`)))
    (`SGameModeBase.WriteSaveGame` _assgame_mode_base)
    (`KismetSystemLibrary.PrintString` "Save game succed")))

(fn `UserConstructionScript`)