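; BoneFired_BP is an interactable bonfire that lights and saves the game when used.
; Interact sets IsFired, calls WriteSaveGame on SGameModeBase, refreshes the flames and prints a confirmation.
; OnActorLoaded runs the same flame update, which activates the Fire component only if IsFired is true, so the lit state can be shown after loading.
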(event `updateFlames`
  (if (`self.bIsFired`)
    (`ActorComponent.Activate` (`self.fire`) false)))

(event `SGameplayInterface.Interact`
  (params (InstigatorPawn :type "Pawn Object Reference"))
  (set `self.bIsFired` true)
  (bind _assgame_mode_base (cast `SGameModeBase` (`GameplayStatics.GetGameMode`)))
  (`SGameModeBase.WriteSaveGame` _assgame_mode_base)
  (`self.updateFlames`)
  (`KismetSystemLibrary.PrintString` "gamed saved"))

(event `SGameplayInterface.OnActorLoaded`
  (`self.updateFlames`))

(fn `UserConstructionScript`)