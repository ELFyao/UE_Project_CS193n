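; Sprint action Blueprint that raises the instigator's walk speed while the action runs.
; On start, it adds a SprintAcceleration amount to the Max Walk Speed of the instigator's Character Movement Component.
; On stop, it subtracts the same variable, reversing the boost additively rather than restoring a cached speed.
; Both events call the parent action first and skip the change if no movement component is found.
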(event `self.StartAction`
  (params (InstigatorActor :type "Actor Object Reference"))
  (bind _returnvalue (`Actor.GetComponentByClass` InstigatorActor "/Script/Engine.CharacterMovementComponent"))
  (`parent.StartAction` InstigatorActor)
  (`/Engine/EditorBlueprintResources/StandardMacros.IsValid` _returnvalue
    (:`Is Valid`
      (set `CharacterMovementComponent.MaxWalkSpeed` (+ (`CharacterMovementComponent.MaxWalkSpeed` _returnvalue) (`self.SprintAcceleration`)) _returnvalue))))

(event `self.StopAction`
  (params (InstigatorActor :type "Actor Object Reference"))
  (bind _returnvalue (`Actor.GetComponentByClass` InstigatorActor "/Script/Engine.CharacterMovementComponent"))
  (`parent.StopAction` InstigatorActor)
  (`/Engine/EditorBlueprintResources/StandardMacros.IsValid` _returnvalue
    (:`Is Valid`
      (set `CharacterMovementComponent.MaxWalkSpeed` (- (`CharacterMovementComponent.MaxWalkSpeed` _returnvalue) (`self.SprintAcceleration`)) _returnvalue))))