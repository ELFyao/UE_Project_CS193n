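; Black hole projectile that applies gravity to its surroundings and destroys what it touches.
; It fires a RadialForce impulse every tick, and any actor that begins overlapping its Sphere is destroyed with no filtering.
; A timer set on BeginPlay destroys the projectile after a few seconds.
; A fallback node to make the Sphere ignore the instigator when moving is left unconnected.
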(event `self.ReceiveTick`
  (params (DeltaSeconds :type "Float (single-precision)"))
  ;[1 1 1] blackhole gravitition
  (`RadialForceComponent.FireImpulse` (`self.RadialForce`)))

(event `self.ReceiveBeginPlay`
  ;[1 1 1] timer to detroy self
  (`KismetSystemLibrary.K2_SetTimerDelegate` (delegate `destroy`) 5.0))

(event `destroy`
  ;[1 1 1] timer to detroy self
  (`self.K2_DestroyActor` self))

(event `self.Sphere.OnComponentBeginOverlap`
  (params (OverlappedComponent :type "PrimitiveComponent Object Reference") (OtherActor :type "Actor Object Reference") (OtherComp :type "PrimitiveComponent Object Reference") (OtherBodyIndex :type Integer) (bFromSweep :type Boolean) (SweepResult :type "HitResult Structure (by ref)"))
  ;[1 1 1] crash other actor to piece
  (`self.K2_DestroyActor` OtherActor))

(fn `UserConstructionScript`)